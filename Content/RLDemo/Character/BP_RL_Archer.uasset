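; BP_RL_Archer is a character Blueprint in RLDemo that handles weapon switching and the matching animation style.
; BeginPlay links the normal animation layers and sets the movement state to Jogging.
; The weapon-change input maps its value to fists, one-handed weapon, magic or bow, setting EquipedWeapon and linking that anim class layer; a note marks this for later C++ implementation.
; Holding the Subtract key slows global time.
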(event Input|EnhancedActionEvents|EnhancedInputActionIA_ChangeWeapon
  (params (ActionValue :type Float%20%28double-precision%29) (ElapsedSeconds :type Float%20%28double-precision%29) (TriggeredSeconds :type Float%20%28double-precision%29) (InputAction :type Input%20Action%20Object%20Reference :default "/Game/RLDemo/Controller/Input/Actions/IA_ChangeWeapon.IA_ChangeWeapon"))
  (bind _mesh (Variables|Character|GetMesh))
  ;[0 0.7544 1] 切换武器，之后会在C++实现
  (:Started
    (switch int (Math|Float|Truncate ActionValue)
      (:1
        (Variables|Default|SetEquipedWeapon "Fists")
        (Components|SkeletalMesh|AnimationBlueprintLinking|LinkAnimClassLayers _mesh "/Game/RLDemo/ABP/ABP_Normal.ABP_Normal_C"))
      (:2
        (Variables|Default|SetEquipedWeapon "OneHandWeapon")
        (Components|SkeletalMesh|AnimationBlueprintLinking|LinkAnimClassLayers _mesh "/Game/RLDemo/ABP/ABP_OnHandWeapon.ABP_OnHandWeapon_C"))
      (:3
        (Variables|Default|SetEquipedWeapon "Magic")
        (Components|SkeletalMesh|AnimationBlueprintLinking|LinkAnimClassLayers _mesh "/Game/RLDemo/ABP/ABP_Magic.ABP_Magic_C"))
      (:4
        (Variables|Default|SetEquipedWeapon "Bow")
        (Components|SkeletalMesh|AnimationBlueprintLinking|LinkAnimClassLayers _mesh "/Game/RLDemo/ABP/ABP_Bow.ABP_Bow_C")))))

(event EventBeginPlay
  (Components|SkeletalMesh|AnimationBlueprintLinking|LinkAnimClassLayers (Variables|Character|GetMesh) "/Game/RLDemo/ABP/ABP_Normal.ABP_Normal_C")
  (Class|RLBaseCharacter|UpdateMovementState "Jogging"))

(event Collision|EventActorBeginOverlap
  (params (OtherActor :type Actor%20Object%20Reference)))

(event EventTick
  (params (DeltaSeconds :type Float%20%28single-precision%29)))

(event Input|KeyboardEvents|Subtract
  (params (Key :type Key%20Structure :default "None"))
  (:Pressed
    (Utilities|Time|SetGlobalTimeDilation 0.1))
  (:Released
    (Utilities|Time|SetGlobalTimeDilation 1.0)))

(fn ConstructionScript)