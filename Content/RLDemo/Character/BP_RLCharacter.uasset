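; Player character Blueprint for the RLDemo game, handling weapon equipping, rolling, jumping and death animation.
; BeginPlay equips the one-hand weapon and notifies the AnimInstance; weapon switches link one- or two-hand anim class layers.
; Roll jumps once if allowed, otherwise turns toward movement input and plays a montage unless one is already playing.
; It also sets a motion-warping facing target, and an Alt+1 debug key grants souls through PlayerState.
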(event EventBeginPlay
  (Utilities|FlowControl|Sequence
    (:then_0
      (Components|SkeletalMesh|AnimationBlueprintLinking|LinkAnimClassLayers (Variables|Character|GetMesh) "/Game/RLDemo/Anim/AnimationBlueprint/Layers/ABP_OnHandWeapon.ABP_OnHandWeapon_C"))
    (:then_1
      (Variables|Default|SetEquipedWeapon "OneHandWeapon")
      (Variables|Default|SetbHasWeapon true)
      (Class|BPICharacterBaseAnim|ReciveEquipWeapon(Message) (Components|SkeletalMesh|GetAnimInstance (Variables|Character|GetMesh)) (Variables|Default|GetEquipedWeapon) (Variables|Default|GetbHasWeapon)))
    (:then_2
      (bind _asbp_player_state (Utilities|Casting|CastToBP_PlayerState (Game|GetPlayerState 0)))
      (Variables|Default|SetAs%20BP%20Player%20State _asbp_player_state))))

(event EventSetFacingTarget
  (params (TargetLoction :type Vector :default "0, 0, 0") (TargetRotation :type Rotator :default "0, 0, 0") (Offest :type Float%20%28single-precision%29))
  (Class|MotionWarpingComponent|AddorUpdateWarpTargetfromLocation (Variables|Default|GetMotionWarping) "FacingTarget" TargetLoction))

(event EventOnDead
  (Class|BPICharacterBaseAnim|RecivebIsDead(Message) (Components|SkeletalMesh|GetAnimInstance (Variables|Character|GetMesh)) (Variables|Default|GetbIsDead)))

(event EventOnSwitchWeapon
  (params (InWeaponType :type E_WeaponType%20Enum :default "Sword"))
  (switch Utilities|FlowControl|Switch|SwitchonE_WeaponType InWeaponType
    (:Sword
      (Components|SkeletalMesh|AnimationBlueprintLinking|LinkAnimClassLayers (Variables|Character|GetMesh) "/Game/RLDemo/Anim/AnimationBlueprint/Layers/ABP_OnHandWeapon.ABP_OnHandWeapon_C"))
    (:GreatSword
      (Components|SkeletalMesh|AnimationBlueprintLinking|LinkAnimClassLayers (Variables|Character|GetMesh) "/Game/RLDemo/Anim/AnimationBlueprint/Layers/ABP_TwoHandWeapon.ABP_TwoHandWeapon_C"))))

(event Input|KeyboardEvents|Alt1
  (params (Key :type Key%20Structure :default "None"))
  (:Pressed
    (Class|RLPlayerState|SetSoul (Variables|Default|GetAs%20BP%20Player%20State) 9999999)))

(fn ConstructionScript)

(fn PlayPriorityMontage
  (params (Montage :type Anim%20Montage%20Object%20Reference))
  (if (not (Class|AnimInstance|IsAnyMontagePlaying (Components|SkeletalMesh|GetAnimInstance (Variables|Character|GetMesh))))
    (Animation|PlayAnimMontage Montage 1.0 "None")))

(fn Roll
  (if (Variables|Default|GetCanJump?)
    ;[1 1 1] 只能跳跃一次
    (Character|Jump)
    (Utilities|Time|ClearandInvalidateTimerbyHandle (Variables|Default|GetJumpTimer))
    (Variables|Default|SetAfterRunTime 0.0)
    (Variables|Default|SetCanJump? false)
    (elif (Math|Vector|VectorIsNearlyZero (Class|Pawn|GetLastMovementInputVector))
      (CallFunction|PlayPriorityMontage)
      (else
        (Transformation|SetActorRotation (Math|Conversions|RotationFromXVector (Class|Pawn|GetLastMovementInputVector)))
        (CallFunction|PlayPriorityMontage)))))