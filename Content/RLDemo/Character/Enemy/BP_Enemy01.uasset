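; BP_Enemy01 is an enemy Blueprint that, so far, only reports its distance to the player as debug text.
; Tick casts player character 0 to BP_RLCharacter and accumulates delta time in a Float variable, printing the distance and resetting the timer about every half second.
; BeginPlay and overlap events are disabled placeholders, and the construction script only calls its parent.
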(event EventBeginPlay
  (|CallParentFunction) ; 此节点被禁用，将不会被调用。\n从引脚连出引线来编译功能。
)

(event Collision|EventActorBeginOverlap
  (params (OtherActor :type Actor%20Object%20Reference)))

(event EventTick
  (params (DeltaSeconds :type Float%20%28single-precision%29))
  (bind _asbp_rlcharacter (Utilities|Casting|CastToBP_RLCharacter (Game|GetPlayerCharacter 0)))
  (if (>= (Variables|Default|Getfloat) 0.5)
    (Development|PrintString (Utilities|String|ToString(Float) (Math|Vector|Distance(Vector) (Transformation|GetActorLocation _asbp_rlcharacter) (Transformation|GetActorLocation))))
    (Variables|Default|Setfloat 0.0)
    (else
      (Variables|Default|Setfloat (+ (Utilities|Time|GetWorldDeltaSeconds) (Variables|Default|Getfloat))))))

(fn ConstructionScript
  (|CallParentFunction))