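; Base enemy Blueprint for RLDemo, handling lock-on display, boss health bar, attack-facing warp and soul reward.
; BeginPlay links two-hand-weapon anim layers, creates the boss widget and binds lock changes to a socket-attached marker.
; SetFacingTarget feeds an offset-adjusted motion-warp target, and a timeline applies the resilience-restore GameplayEffect each update.
; DropSouls credits the player directly through an interface; physics bone-shake and soul-pickup spawning are disconnected.
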(event Custom|OnLock_事件
  (params (bLock :type Boolean))
  (Rendering|SetVisibility (Variables|Default|GetLockUIWidgetComponnet) bLock false))

(event EventBeginPlay
  (Utilities|FlowControl|Sequence
    (:then_0
      (Components|SkeletalMesh|AnimationBlueprintLinking|LinkAnimClassLayers (Variables|Character|GetMesh) "/Game/RLDemo/Anim/AnimationBlueprint/Layers/ABP_TwoHandWeapon.ABP_TwoHandWeapon_C")
      (bind _returnvalue (UserInterface|CreateWidget (Variables|Enemy|GetBossWidget)))
      (bind _output_get (Variables|Enemy|SetBossHealthWidget _returnvalue))
      (Utilities|IsValid _output_get
        (:Is%20Valid
          (Class|RLUserWidget|SetWidgetController (Variables|Enemy|GetBossHealthWidget) self 0))))
    (:then_1
      (EventDispatchers|AssignOnLock (delegate Custom|OnLock_事件)))))

(event EventSetFacingTarget
  (params (TargetLoction :type Vector :default "0, 0, 0") (TargetRotation :type Rotator :default "0, 0, 0") (Offest :type Float%20%28single-precision%29))
  (CallFunction|SetMotionWrap TargetLoction Offest))

(event EventResilienceReduceCallBack
  (bind _abilitysystemcomponent (Variables|Default|GetAbilitySystemComponent))
  (Timeline|ResilienceReduce PlayFromStart
    (:Update
      (GameplayEffects|ApplyGameplayEffectToSelf _abilitysystemcomponent "/Game/RLDemo/GAS/Effect/ChangeAttribute/EnemyState/GE_RestoreResilience.GE_RestoreResilience_C" 1.0 (GameplayEffects|MakeEffectContext _abilitysystemcomponent)))))

(event EventPlayBoneShake
  (params (BoneName :type Name :default "None") (ShakeDirection :type Vector :default "0, 0, 0") (Magnitude :type Float%20%28single-precision%29))
  ;[1 1 1] 局部骨骼抖动
)

(event EventDropSouls
  (bind _targetactor (Variables|Default|GetTargetActor))
  (if (Utilities|DoesObjectImplementInterface _targetactor "/Script/UE_RougelikeDemo.RL_PlayerInterface")
    (Class|RLPlayerInterface|AddSoul(Message) _targetactor (Variables|/Script/UE_RougelikeDemo.RL_EnemyConfig|GetSoulCount (Variables|/Script/UE_RougelikeDemo.RL_EnemyMovementComponent|GetEnemyConfig (Variables|Default|GetEnemyMovementComponent))))
    (Utilities|IsValid (Variables|Enemy|GetBossHealthWidget)
      (:Is%20Valid
        (Widget|RemovefromParent (Variables|Enemy|GetBossHealthWidget))
        (Variables|Enemy|SetBossHealthWidget 0)))))

(event EventShowBossHealthBar
  (params (bVisible :type Boolean))
  (Utilities|IsValid (Variables|Enemy|GetBossHealthWidget)
    (:Is%20Valid
      (if bVisible
        (UserInterface|Viewport|AddtoViewport (Variables|Enemy|GetBossHealthWidget) 0)
        (Development|SetHiddeninGame (Variables|Default|GetHealthBar) true true)
        (else
          (Widget|RemovefromParent (Variables|Enemy|GetBossHealthWidget)))))))

(fn ConstructionScript
  (Transformation|AttachComponentToComponent (Variables|Default|GetLockUIWidgetComponnet) (Variables|Character|GetMesh) (Variables|Enemy|GetLockUIAttachedSocketName) "KeepRelative" "KeepRelative" "KeepRelative" true))

(fn SetMotionWrap
  (params (Target%20Loction :type Vector) (Offest :type Float%20%28double-precision%29))
  (bind _returnvalue (Transformation|GetActorLocation))
  (bind _returnvalue_2 (- Target%20Loction _returnvalue))
  ;[1 1 1] 计算偏移位置
  (LocalVariables|SetDirectionVec (Math|Vector|Normalize _returnvalue_2))
  (bind _output_get (LocalVariables|SetInOffest (- (Math|Vector|VectorLength _returnvalue_2) Offest)))
  (if (> _output_get 0.0)
    (Class|MotionWarpingComponent|AddorUpdateWarpTargetfromLocationandRotation (Variables|Default|GetMotionWarping) "FacingTarget" (+ (* (* (LocalVariables|GetDirectionVec) (LocalVariables|GetInOffest)) "1.000000,1.000000,0.000000") (Transformation|GetActorLocation)) (Math|Rotator|FindLookatRotation (Transformation|GetActorLocation) Target%20Loction))))