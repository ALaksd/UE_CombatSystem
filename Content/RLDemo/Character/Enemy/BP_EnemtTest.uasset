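; Test enemy character that arms itself with a two-handed weapon setup on BeginPlay.
; It links the two-handed weapon anim layers, sets RLMovement to Jogging and notifies the AnimInstance of the equipped weapon.
; It then generates a sword item instance from its data asset through the RL inventory subsystem and loots it into the equipment inventory component.
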(event EventBeginPlay
  (Utilities|FlowControl|Sequence
    (:then_0
      (Components|SkeletalMesh|AnimationBlueprintLinking|LinkAnimClassLayers (Variables|Character|GetMesh) "/Game/RLDemo/Anim/AnimationBlueprint/Layers/ABP_TwoHandWeapon.ABP_TwoHandWeapon_C")
      (Class|RLMovementComponent|UpdateMovementState (Variables|Default|GetRL_Movement) "Jogging")
      (Class|BPICharacterBaseAnim|ReciveEquipWeapon(Message) (Components|SkeletalMesh|GetAnimInstance (Variables|Character|GetMesh)) "TwoHandedWeapon" true))
    (:then_1
      (bind _returnvalue (Class|RLInventorySubsystem|GenerateItemInstance (Subsystems|GetRLInventorySubsystem) "/Game/RLDemo/Item/DA_Weapon_Sword_01.DA_Weapon_Sword_01"))
      (Class|RLInventoryComponent|LootItem (Variables|Default|GetRLInventoryComponent_Equipment) _returnvalue))))

(fn ConstructionScript)