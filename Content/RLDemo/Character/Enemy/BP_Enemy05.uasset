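; BP_Enemy05 is an enemy character Blueprint built from several skeletal mesh parts that animate as one body.
; On BeginPlay it sets the main Mesh as leader pose component for four additional skeletal meshes, so they follow its pose.
; A SetMeshLeader function repeats the same binding but is not called within this Blueprint, and the construction script is empty.
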(event EventBeginPlay
  (Components|SkinnedMesh|SetLeaderPoseComponent (Variables|Default|GetSkeletalMesh3) (Variables|Character|GetMesh) false false))

(fn ConstructionScript)

(fn SetMeshLeader
  (Components|SkinnedMesh|SetLeaderPoseComponent (Variables|Default|GetSkeletalMesh3) (Variables|Character|GetMesh) false false)
  (Components|SkinnedMesh|SetLeaderPoseComponent (Variables|Default|GetSkeletalMesh2) (Variables|Character|GetMesh) false false)
  (Components|SkinnedMesh|SetLeaderPoseComponent (Variables|Default|GetSkeletalMesh1) (Variables|Character|GetMesh) false false)
  (Components|SkinnedMesh|SetLeaderPoseComponent (Variables|Default|GetSkeletalMesh) (Variables|Character|GetMesh) false false))