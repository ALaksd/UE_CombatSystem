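; BP_Boss02_1 is the first form of the Boss02 enemy, handing off to BP_Boss02_2 when it drops souls.
; DropSouls runs the parent logic, plays the Boss2_2 level sequence and, after a fixed delay, spawns the next form above its position.
; The spawned boss gets a level and default controller, then background music fades to the Boss2_2 track.
; The construction script attaches the Hair component to the mesh's Hair socket.
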(event EventBeginPlay
  (|CallParentFunction) ; 此节点被禁用，将不会被调用。\n从引脚连出引线来编译功能。
)

(event Collision|EventActorBeginOverlap
  (params (OtherActor :type Actor%20Object%20Reference)))

(event EventTick
  (params (DeltaSeconds :type Float%20%28single-precision%29)))

(event EventDropSouls
  (bind _returnvalue (Transformation|GetActorTransform))
  (bind (_location _rotation _scale) (Math|Transform|BreakTransform _returnvalue))
  (bind (_x _y _z) (Math|Vector|BreakVector _location))
  (|CallParentFunction)
  (bind _returnvalue_2 (Sequencer|Player|CreateLevelSequencePlayer "/Game/RLDemo/v/boss2_2.boss2_2"))
  (Utilities|IsValid _returnvalue_2
    (:Is%20Valid
      (Sequencer|Player|Play _returnvalue_2 :!class /Script/MovieScene.MovieSceneSequencePlayer))
    (:Is%20Not%20Valid
      _))
  (Utilities|FlowControl|Delay 5.0)
  (bind _returnvalue_3 (Game|SpawnActorfromClass "/Game/RLDemo/Character/Enemy/BP_Boss02_2.BP_Boss02_2_C" (Math|Transform|MakeTransform (Math|Vector|MakeVector _x _y (+ _z 5e+02)) _rotation _scale) "Undefined" "MultiplyWithRoot" 0 0))
  (Class|RLEnemyInterface|SetEnemyLevel _returnvalue_3 5)
  (Pawn|SpawnDefaultController _returnvalue_3)
  (Class|RLMusicSubSystem|PlayBackgroundMusic (Subsystems|GetRLMusicSubSystem) "/Game/RLDemo/Sound/BGM_Boss2_2.BGM_Boss2_2" 1.0))

(fn ConstructionScript
  (|CallParentFunction)
  (Transformation|AttachComponentToComponent (Variables|Default|GetHair) (Variables|Character|GetMesh) "Hair" "KeepRelative" "KeepRelative" "KeepRelative" true))