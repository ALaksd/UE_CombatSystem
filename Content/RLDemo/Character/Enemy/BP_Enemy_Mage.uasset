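; Mage enemy character Blueprint that repeatedly plays a fireball casting animation.
; On BeginPlay, SetMeshLeader makes four extra skeletal mesh parts follow the main Mesh through leader pose.
; It then plays FireBall_Montage on Mesh, and each completion waits briefly, prints a debug "Fire" message and replays the montage.
; The file shows no projectile spawning, targeting or AI logic.
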(event EventBeginPlay
  (CallFunction|SetMeshLeader)
  (Animation|Montage|PlayMontage (Variables|Character|GetMesh) "/Game/RLDemo/Anim/AnimMontage/Enemy/Mage/FireBall_Montage.FireBall_Montage" :!label _label
    (:OnCompleted
      (Utilities|FlowControl|Delay 2.0)
      (Development|PrintString "Fire" true true "(R=0.037924,G=1.000000,B=0.000000,A=1.000000)")
      (goto _label))))

(fn ConstructionScript)

(fn SetMeshLeader
  (Components|SkinnedMesh|SetLeaderPoseComponent (Variables|Default|GetSkeletalMesh3) (Variables|Character|GetMesh) false false)
  (Components|SkinnedMesh|SetLeaderPoseComponent (Variables|Default|GetSkeletalMesh2) (Variables|Character|GetMesh) false false)
  (Components|SkinnedMesh|SetLeaderPoseComponent (Variables|Default|GetSkeletalMesh1) (Variables|Character|GetMesh) false false)
  (Components|SkinnedMesh|SetLeaderPoseComponent (Variables|Default|GetSkeletalMesh) (Variables|Character|GetMesh) false false))