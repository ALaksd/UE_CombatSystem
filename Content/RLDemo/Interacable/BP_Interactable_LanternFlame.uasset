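; BP_Interactable_LanternFlame is an interactable lantern flame that serves as a save point.
; InitPointName casts the WBPSavePoint widget to WBP_SavePoint and sets its PointName from LanternFlameName.
; OnPointActivaete starts the Niagara effect and adds a WBP_SavePonitActiveMessage widget to the viewport to announce the activation.
; The graph holds no save logic of its own, and BeginPlay, overlap and Tick do nothing.
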(event EventBeginPlay)

(event Collision|EventActorBeginOverlap
  (params (OtherActor :type Actor%20Object%20Reference)))

(event EventTick
  (params (DeltaSeconds :type Float%20%28single-precision%29)))

(event EventInitPointName
  (Utilities|IsValid (Variables|Default|GetWBP_SavePoint)
    (:Is%20Valid
      (bind _aswbp_save_point (Utilities|Casting|CastToWBP_SavePoint (Variables|Default|GetWBP_SavePoint)))
      (Variables|/Game/RLDemo/UI/Widget/LanternFlame/WBP_SavePoint.WBP_SavePoint_C|SetPointName _aswbp_save_point (Utilities|Text|ToText(String) (Variables|Default|GetLanternFlameName))))))

(event EventOnPointActivaete
  (Components|Activation|Activate (Variables|Default|GetNiagara) false)
  (bind _returnvalue (UserInterface|CreateWidget "/Game/RLDemo/UI/Widget/LanternFlame/WBP_SavePonitActiveMessage.WBP_SavePonitActiveMessage_C"))
  (UserInterface|Viewport|AddtoViewport _returnvalue 0))

(fn ConstructionScript)