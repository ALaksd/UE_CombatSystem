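; BP_PlayerState is the demo's player state Blueprint, wired as a test harness for the inventory and equipment system.
; Shortly after BeginPlay, it has the RLInventorySubsystem generate an item instance from DA_EquipTest and loots it into the equipment inventory component, printing a debug message on success.
; Every Tick, it prints the name of the item in the first slot of the separate InventoryComponent.
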(event EventBeginPlay
  (Utilities|FlowControl|Delay 2.0)
  (bind _returnvalue (Class|RLInventorySubsystem|GenerateItemInstance (Subsystems|GetRLInventorySubsystem) "/Game/RLDemo/Item/DA_EquipTest.DA_EquipTest"))
  (bind _returnvalue_2 (Class|RLInventoryComponent|LootItem (Variables|Default|GetEquipmentInventoryComponnet) _returnvalue))
  (if _returnvalue_2
    (Development|PrintString "Hello")))

(event EventTick
  (params (DeltaSeconds :type Float%20%28single-precision%29))
  (bind _inventorycomponent (Variables|Default|GetInventoryComponent))
  (bind _returnvalue (Class|RLInventoryComponent|GetItemInstanceinSlot _inventorycomponent (Utilities|Array|Get(acopy) (Class|RLInventoryComponent|GetAllSlotHandles _inventorycomponent))))
  (Development|PrintString (Utilities|GetObjectName _returnvalue) true true "(R=0.000000,G=0.660000,B=1.000000,A=1.000000)" 1.0 "1"))

(fn ConstructionScript)