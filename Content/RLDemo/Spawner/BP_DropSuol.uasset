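; BP_DropSuol is a soul pickup that passes its soul count to the player when touched.
; Its construction script sets the ProjectileMovement homing target to the root component of HomingTarget.
; On sphere overlap, it calls AddSoulMessage on any actor implementing RL_PlayerInterface, then destroys itself.
; Manual target lookup and movement logic remains in the event graph but is disconnected, and Tick does nothing.
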(event OnComponentBeginOverlap(Sphere)
  (params (OverlappedComponent :type Primitive%20Component%20Object%20Reference) (OtherActor :type Actor%20Object%20Reference) (OtherComp :type Primitive%20Component%20Object%20Reference) (OtherBodyIndex :type Integer) (bFromSweep :type Boolean) (SweepResult :type Hit%20Result%20Structure%20%28by%20ref%29))
  (if (Utilities|DoesObjectImplementInterface OtherActor "/Script/UE_RougelikeDemo.RL_PlayerInterface")
    (Class|RLPlayerInterface|AddSoul(Message) OtherActor (Variables|Default|GetSoulCount))
    (Actor|DestroyActor)))

(event EventBeginPlay)

(event Collision|EventActorBeginOverlap
  (params (OtherActor :type Actor%20Object%20Reference)))

(event EventTick
  (params (DeltaSeconds :type Float%20%28single-precision%29)))

(fn ConstructionScript
  (Variables|/Script/Engine.ProjectileMovementComponent|SetHomingTargetComponent (Variables|Default|GetProjectileMovement) (Variables|/Script/Engine.Actor|GetRootComponent (Variables|Default|GetHomingTarget))))